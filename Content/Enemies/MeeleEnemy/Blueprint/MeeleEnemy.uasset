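; Melee enemy AI that patrols random points around a center and chases the player when perception senses them.
; Reaching the player sets attack state and a random attack index, while switchable hand hitboxes deal interface-based damage, tracking hit actors to avoid repeats.
; Taking damage slows it and sets hurt or dead flags, with destruction in a separate event.
; Its health bar shows within a proximity sphere and is re-oriented every tick.
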(event OnTargetPerceptionUpdated(AIPerception)
  (params (Actor :type Actor%20Object%20Reference) (Stimulus :type AI%20Stimulus%20Structure))
  ;[1 1 1] Perseguir
  (if (not (Variables|Combat|GetIsDead))
    (if (and (== Actor (Game|Player|GetPlayerPawn 0)) (.bSuccessfullySensed (Utilities|Struct|BreakAIStimulus Stimulus)))
      (Variables|/Script/Engine.CharacterMovementComponent|SetMaxWalkSpeed (Variables|Character|GetCharacterMovement) (Variables|Movement|GetRunSpeed))
      (AI|AIMoveTo self "0, 0, 0" (Game|Player|GetPlayerPawn 0) 7e+01 false
        (:OnSuccess
          (Variables|Combat|SetIsAttacking true)
          (Variables|Combat|SetAttackIndex (Math|Random|RandomIntegerinRange 0 1))
          (Variables|/Script/Engine.CharacterMovementComponent|SetMaxWalkSpeed (Variables|Character|GetCharacterMovement) (Variables|Movement|GetDamagedSpeed)))
        (:OnFail
          (CallFunction|Patrol (Transformation|GetActorLocation (Variables|Patrol|GetPatrolCenter)) :!label _label)))
      (else
        (goto _label)))))

(event OnComponentBeginOverlap(RHBox)
  (params (OverlappedComponent :type Primitive%20Component%20Object%20Reference) (OtherActor :type Actor%20Object%20Reference) (OtherComp :type Primitive%20Component%20Object%20Reference) (OtherBodyIndex :type Integer) (bFromSweep :type Boolean) (SweepResult :type Hit%20Result%20Structure%20%28by%20ref%29))
  ;[1 1 1] Hit
  (CallFunction|Hit OtherActor))

(event OnComponentBeginOverlap(LHBox)
  (params (OverlappedComponent :type Primitive%20Component%20Object%20Reference) (OtherActor :type Actor%20Object%20Reference) (OtherComp :type Primitive%20Component%20Object%20Reference) (OtherBodyIndex :type Integer) (bFromSweep :type Boolean) (SweepResult :type Hit%20Result%20Structure%20%28by%20ref%29))
  ;[1 1 1] Hit
  (CallFunction|Hit OtherActor))

(event OnComponentBeginOverlap(Sphere)
  (params (OverlappedComponent :type Primitive%20Component%20Object%20Reference) (OtherActor :type Actor%20Object%20Reference) (OtherComp :type Primitive%20Component%20Object%20Reference) (OtherBodyIndex :type Integer) (bFromSweep :type Boolean) (SweepResult :type Hit%20Result%20Structure%20%28by%20ref%29))
  ;[1 1 1] Toggle health bar
  (if (== OtherActor (.AsPlayer (Utilities|Casting|CastToPlayer OtherActor)))
    (Rendering|SetVisibility (Variables|Default|GetHealthBar) true true)))

(event OnComponentEndOverlap(Sphere)
  (params (OverlappedComponent :type Primitive%20Component%20Object%20Reference) (OtherActor :type Actor%20Object%20Reference) (OtherComp :type Primitive%20Component%20Object%20Reference) (OtherBodyIndex :type Integer))
  ;[1 1 1] Toggle health bar
  (if (== OtherActor (.AsPlayer (Utilities|Casting|CastToPlayer OtherActor)))
    (Rendering|SetVisibility (Variables|Default|GetHealthBar) false false)))

(event Custom|Patrol
  (params (Position :type Vector))
  ;[1 1 1] Patrullar
  (Variables|/Script/Engine.CharacterMovementComponent|SetMaxWalkSpeed (Variables|Character|GetCharacterMovement) (Variables|Movement|GetWalkSpeed))
  (if (not (or (Variables|Combat|GetIsDead) (Variables|Combat|GetIsGettigDamage)))
    (AI|AIMoveTo self Position 0 5e+01 false
      (:OnSuccess
        (CallFunction|Patrol (.RandomLocation (AI|Navigation|GetRandomReachablePointinRadius (Transformation|GetActorLocation (Variables|Patrol|GetPatrolCenter)) (Variables|Patrol|GetPatrolRadius) 0 0)))))))

(event Custom|DisableBothHandsCollision
  ;[1 1 1] Disable / Enable Hands Collision
  ;;[1 1 1] Disable Both
  (Collision|SetCollisionEnabled (Variables|Default|GetRHBox) "NoCollision")
  (Collision|SetCollisionEnabled (Variables|Default|GetLHBox) "NoCollision"))

(event Custom|DisableRightHandCollision
  ;[1 1 1] Disable / Enable Hands Collision
  ;;[1 1 1] Disable / Enable Right Hand
  (Collision|SetCollisionEnabled (Variables|Default|GetRHBox) "NoCollision")
  (Utilities|Array|Clear (Variables|Combat|GetEnemiesHit)))

(event Custom|DisableLeftHandCollision
  ;[1 1 1] Disable / Enable Hands Collision
  ;;[1 1 1] Disable / Enable Left Hand
  (Collision|SetCollisionEnabled (Variables|Default|GetLHBox) "NoCollision")
  (Utilities|Array|Clear (Variables|Combat|GetEnemiesHit)))

(event Custom|EnableRightHandCollision
  ;[1 1 1] Disable / Enable Hands Collision
  ;;[1 1 1] Disable / Enable Right Hand
  (Collision|SetCollisionEnabled (Variables|Default|GetRHBox) "QueryOnly"))

(event Custom|EnableLeftHandCollision
  ;[1 1 1] Disable / Enable Hands Collision
  ;;[1 1 1] Disable / Enable Left Hand
  (Collision|SetCollisionEnabled (Variables|Default|GetLHBox) "QueryOnly"))

(event Custom|Dead
  ;[1 1 1] Dead
  (Actor|DestroyActor))

(event EventDamage
  (params (Damage :type Float%20%28double-precision%29))
  ;[1 1 1] Get damage
  (Variables|Combat|SetHealth (- (Variables|Combat|GetHealth) Damage))
  (Variables|/Script/Engine.CharacterMovementComponent|SetMaxWalkSpeed (Variables|Character|GetCharacterMovement) (Variables|Movement|GetDamagedSpeed))
  (if (<= (Variables|Combat|GetHealth) 0.0)
    (CallFunction|UpdateHealthBar)
    (Variables|Combat|SetIsDead true)
    (else
      (CallFunction|UpdateHealthBar)
      (Variables|Combat|SetIsGettigDamage true))))

(event EventTick
  (params (DeltaSeconds :type Float%20%28single-precision%29))
  ;[1 1 1] Event tick
  (Transformation|SetWorldRotation (Variables|Default|GetHealthBar) (|SetHealthBarrotationtoPlayerCamera) false false))

(event EventBeginPlay
  ;[1 1 1] Begin Play
  (Variables|Combat|SetHealth (Variables|Combat|GetMaxHealth))
  (CallFunction|DisableBothHandsCollision)
  (Utilities|FlowControl|Sequence
    (:then_0
      (if (not (Variables|Combat|GetIsDead))
        (CallFunction|Patrol (Transformation|GetActorLocation (Variables|Patrol|GetPatrolCenter)))))
    (:then_1
      (CallFunction|UpdateHealthBar)
      (Rendering|SetVisibility (Variables|Default|GetHealthBar) false false))))

(fn ConstructionScript)

(fn Hit
  (params (OtherActor :type Actor%20Object%20Reference))
  (if (== OtherActor (Game|Player|GetPlayerPawn 0))
    (if (not (Utilities|Array|ContainsItem (Variables|Combat|GetEnemiesHit) OtherActor))
      (if (Utilities|DoesObjectImplementInterface OtherActor "/Game/BluePrintInterfaces/BPI_Damageable.BPI_Damageable_C")
        (Utilities|Array|Add (Variables|Combat|GetEnemiesHit) OtherActor)
        (Class|BPIDamageable|ReceiveDamage(Message) OtherActor (Variables|Combat|GetDamage))))))

(fn UpdateHealthBar
  (Variables|/Game/Enemies/MeeleEnemy/UI/WBP_HealthBar.WBP_HealthBar_C|SetHealthPercent (.AsWBP%20Health%20Bar (Utilities|Casting|CastToWBP_HealthBar (UserInterface|GetUserWidgetObject (Variables|Default|GetHealthBar)))) (/ (Variables|Combat|GetHealth) (Variables|Combat|GetMaxHealth))))